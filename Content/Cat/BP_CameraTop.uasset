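; BP_CameraTop is a top-view camera that pans when the mouse cursor nears the screen edges.
; MouseX and MouseY events compare cursor position to viewport size, using the outer 15% on each side as scroll zones.
; Horizontal edges set local Y movement and vertical edges set local X.
; Both events feed one shared local offset that applies both components at a fixed step per call, without delta-time scaling.
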(event EventBeginPlay)

(event Collision|EventActorBeginOverlap
  (params (OtherActor :type Actor%20Object%20Reference)))

(event EventTick
  (params (DeltaSeconds :type Float%20%28single-precision%29)))

(event Input|MouseEvents|MouseX
  (params (AxisValue :type Float%20%28single-precision%29))
  (bind _returnvalue (Game|GetPlayerController 0))
  (bind _returnvalue_2 (Viewport|GetViewportSize))
  (bind (_locationx _locationy) (Game|Player|GetMousePosition _returnvalue))
  (bind _returnvalue_3 (/ _locationx (.x _returnvalue_2)))
  (if (<= _returnvalue_3 0.15)
    (Variables|Default|SetMovementY -1e+01)
    (elif (>= _returnvalue_3 0.85)
      (Variables|Default|SetMovementY 1e+01)
      (else
        (Variables|Default|SetMovementY 0.0))))
  (Transformation|AddActorLocalOffset (Math|Vector|MakeVector (Variables|Default|GetMovementX) (Variables|Default|GetMovementY) 0.0) false false))

(event Input|MouseEvents|MouseY
  (params (AxisValue :type Float%20%28single-precision%29))
  (bind _returnvalue (Game|GetPlayerController 0))
  (bind _returnvalue_2 (Viewport|GetViewportSize))
  (bind (_locationx _locationy) (Game|Player|GetMousePosition _returnvalue))
  (bind _returnvalue_3 (/ _locationy (.y _returnvalue_2)))
  (if (>= _returnvalue_3 0.85)
    (Variables|Default|SetMovementX -1e+01)
    (elif (<= _returnvalue_3 0.15)
      (Variables|Default|SetMovementX 1e+01)
      (else
        (Variables|Default|SetMovementX 0.0))))
  (Transformation|AddActorLocalOffset (Math|Vector|MakeVector (Variables|Default|GetMovementX) (Variables|Default|GetMovementY) 0.0) false false))

(fn ConstructionScript)