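; Nutrition component, apparently for the cat, that tracks a Food value draining over time.
; On BeginPlay it starts a looping one-second timer that decrements Food while it is above zero and prints the result to screen as debug output.
; FillFood adds a given amount back to Food, with no upper limit.
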(event Custom|FoodConsume
  (bind _food (Variables|Default|GetFood))
  (if (> _food 0.0)
    (bind _result (Math|Float|DecrementFloat _food)
      (:%20%20
        (Development|PrintString (Utilities|String|ToString(Float) _result))))))

(event EventBeginPlay
  (Utilities|Time|SetTimerbyEvent (delegate Custom|FoodConsume) 1.0 true))

(fn FillFood
  (params (FoodAmount :type Float%20%28double-precision%29))
  (Variables|Default|SetFood (+ FoodAmount (Variables|Default|GetFood))))