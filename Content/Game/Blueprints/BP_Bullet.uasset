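; BP_Bullet is a projectile pawn that can be possessed and steered with the mouse during the character's skill.
; With the skill active, it swaps physics and ProjectileMovement for swept per-tick offsets, speeding up if unpossessed or on left click.
; Left click or a Sphere hit returns control to the Character, and unpossessing restores time dilation.
; Sphere hits apply impulses and delay destruction, while StaticMesh hits destroy it immediately.
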(event OnComponentHit(Sphere)
  (params (HitComponent :type Primitive%20Component%20Object%20Reference) (OtherActor :type Actor%20Object%20Reference) (OtherComp :type Primitive%20Component%20Object%20Reference) (NormalImpulse :type Vector :default "0, 0, 0") (Hit :type Hit%20Result%20Structure%20%28by%20ref%29))
  (bind _returnvalue (Game|GetPlayerController 0))
  (if (not (Variables|Default|GetIsHit?))
    (bind _output_get (Variables|Default|SetIsHit? true))
    (Physics|SetSimulatePhysics (Variables|Default|GetStaticMesh) _output_get)
    (Pawn|UnPossess _returnvalue)
    (Pawn|Possess _returnvalue (Variables|Default|GetCharacter))
    (Physics|AddImpulse (Variables|Default|GetStaticMesh) (* (Transformation|GetActorForwardVector) 2e+03) "None" true)
    (if (Physics|IsSimulatingPhysics HitComponent "None")
      (Physics|AddImpulseatLocation HitComponent (* (Transformation|GetVelocity) 2e+03) (Transformation|GetActorLocation) "None"))
    (Utilities|FlowControl|Delay 4.0)
    (Actor|DestroyActor)))

(event OnComponentHit(StaticMesh)
  (params (HitComponent :type Primitive%20Component%20Object%20Reference) (OtherActor :type Actor%20Object%20Reference) (OtherComp :type Primitive%20Component%20Object%20Reference) (NormalImpulse :type Vector :default "0, 0, 0") (Hit :type Hit%20Result%20Structure%20%28by%20ref%29))
  (Development|PrintString "Hello")
  (Actor|DestroyActor))

(event EventBeginPlay
  (bind _staticmesh (Variables|Default|GetStaticMesh))
  (if (Variables|/Game/FirstPerson/Blueprints/BP_FirstPersonCharacter.BP_FirstPersonCharacter_C|GetIsSkillActive (Variables|Default|GetCharacter))
    (Physics|SetSimulatePhysics _staticmesh false)
    (Components|Activation|Deactivate (Variables|Default|GetProjectileMovement))
    (Utilities|FlowControl|Delay 0.5)
    (if (not (Variables|Default|GetIsPossess?))
      (Variables|Default|SetSpeed 6e+02))
    (else
      (Physics|SetSimulatePhysics _staticmesh true))))

(event EventUnpossessed
  (params (OldController :type Controller%20Object%20Reference))
  (Utilities|Time|SetGlobalTimeDilation 1.0))

(event EventTick
  (params (DeltaSeconds :type Float%20%28single-precision%29))
  (if (not (Variables|Default|GetIsHit?))
    (Transformation|AddWorldOffset (Variables|Default|GetSphere) (* (Transformation|GetActorForwardVector) (Variables|Default|GetSpeed)) true false)))

(event EventPossessed
  (params (NewController :type Controller%20Object%20Reference))
  (Variables|Default|SetIsPossess? true))

(event Input|MouseEvents|MouseX
  (params (AxisValue :type Float%20%28single-precision%29))
  (Utilities|FlowControl|Sequence
    (:then_0
      (if (> AxisValue 0.0)
        (Variables|Default|SetMoveR 5.0)
        (Transformation|AddWorldOffset (Variables|Default|GetSphere) (* (Transformation|GetActorRightVector) (Variables|Default|GetMoveR)) true false :!label _label)))
    (:then_1
      (if (< AxisValue 0.0)
        (Variables|Default|SetMoveR -5.0)
        (goto _label)))))

(event Input|MouseEvents|MouseY
  (params (AxisValue :type Float%20%28single-precision%29))
  (Variables|Default|SetMoveUP AxisValue)
  (Utilities|FlowControl|Sequence
    (:then_0
      (if (> AxisValue 0.0)
        (Transformation|AddWorldOffset (Variables|Default|GetSphere) (* (Transformation|GetActorUpVector) (* (Variables|Default|GetMoveUP) 3.0)) true false :!label _label)))
    (:then_1
      (if (< AxisValue 0.0)
        (goto _label)))))

(event Input|MouseEvents|LeftMouseButton
  (params (Key :type Key%20Structure :default "None"))
  (bind _returnvalue (Game|GetPlayerController 0))
  (:Pressed
    (Pawn|UnPossess _returnvalue)
    (Pawn|Possess _returnvalue (Variables|Default|GetCharacter))
    (Variables|Default|SetSpeed 6e+02)))

(fn ConstructionScript)