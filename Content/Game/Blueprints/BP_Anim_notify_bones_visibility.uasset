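; Animation notify state that hides cartridge bones on a six-round weapon mesh, with casings (Gilza) and bullets (Pulya), for part of an animation.
; On begin, it hides all six casing bones and all six bullet bones by hardcoded name on the notifying mesh component.
; On end, it unhides only the casing bones, leaving the bullet bones hidden.
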(fn ReceivedNotifyBegin
  (params (MeshComp :type Skeletal%20Mesh%20Component%20Object%20Reference) (Animation :type Anim%20Sequence%20Base%20Object%20Reference) (TotalDuration :type Float%20%28single-precision%29) (EventReference :type Anim%20Notify%20Event%20Reference%20Structure%20%28by%20ref%29))
  (Components|SkinnedMesh|HideBonebyName MeshComp "Gilza_1_jt" "PBO_None")
  (Components|SkinnedMesh|HideBonebyName MeshComp "Gilza_2_jt" "PBO_None")
  (Components|SkinnedMesh|HideBonebyName MeshComp "Gilza_3_jt" "PBO_None")
  (Components|SkinnedMesh|HideBonebyName MeshComp "Gilza_4_jt" "PBO_None")
  (Components|SkinnedMesh|HideBonebyName MeshComp "Gilza_5_jt" "PBO_None")
  (Components|SkinnedMesh|HideBonebyName MeshComp "Gilza_6_jt" "PBO_None")
  (Components|SkinnedMesh|HideBonebyName MeshComp "Pulya_1_jt1" "PBO_None")
  (Components|SkinnedMesh|HideBonebyName MeshComp "Pulya_2_jt1" "PBO_None")
  (Components|SkinnedMesh|HideBonebyName MeshComp "Pulya_3_jt1" "PBO_None")
  (Components|SkinnedMesh|HideBonebyName MeshComp "Pulya_4_jt1" "PBO_None")
  (Components|SkinnedMesh|HideBonebyName MeshComp "Pulya_5_jt1" "PBO_None")
  (Components|SkinnedMesh|HideBonebyName MeshComp "Pulya_6_jt1" "PBO_None")
  (return false))

(fn ReceivedNotifyEnd
  (params (MeshComp :type Skeletal%20Mesh%20Component%20Object%20Reference) (Animation :type Anim%20Sequence%20Base%20Object%20Reference) (EventReference :type Anim%20Notify%20Event%20Reference%20Structure%20%28by%20ref%29))
  (Components|SkinnedMesh|UnHideBonebyName MeshComp "Gilza_1_jt")
  (Components|SkinnedMesh|UnHideBonebyName MeshComp "Gilza_2_jt")
  (Components|SkinnedMesh|UnHideBonebyName MeshComp "Gilza_3_jt")
  (Components|SkinnedMesh|UnHideBonebyName MeshComp "Gilza_4_jt")
  (Components|SkinnedMesh|UnHideBonebyName MeshComp "Gilza_5_jt")
  (Components|SkinnedMesh|UnHideBonebyName MeshComp "Gilza_6_jt")
  (return false))