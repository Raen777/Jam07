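; BP_Enemy is an enemy that hops and moves toward the player character, damaging it on contact until a bullet disables it.
; While active, a player entering the trigger sphere causes an upward impulse, then a one-second delayed AI move to the player's current location, gated by a resetting DoOnce.
; Collision hits reduce player HP, while a BP_Bullet hit clears IsActive.
; The construction script sizes the trigger; timer-based jump nodes are left unconnected.
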(event OnComponentHit(CollisionComponent)
  (params (HitComponent :type Primitive%20Component%20Object%20Reference) (OtherActor :type Actor%20Object%20Reference) (OtherComp :type Primitive%20Component%20Object%20Reference) (NormalImpulse :type Vector :default "0, 0, 0") (Hit :type Hit%20Result%20Structure%20%28by%20ref%29))
  (Utilities|Casting|CastToBP_Bullet OtherActor
    (:then
      (Variables|Default|SetIsActive false))
    (:CastFailed
      (if (Variables|Default|GetIsActive)
        (bind _asbp_first_person_character (Utilities|Casting|CastToBP_FirstPersonCharacter OtherActor))
        (Default|HPDec _asbp_first_person_character (Variables|Default|GetHPDec))))))

(event OnComponentBeginOverlap(Trigger)
  (params (OverlappedComponent :type Primitive%20Component%20Object%20Reference) (OtherActor :type Actor%20Object%20Reference) (OtherComp :type Primitive%20Component%20Object%20Reference) (OtherBodyIndex :type Integer) (bFromSweep :type Boolean) (SweepResult :type Hit%20Result%20Structure%20%28by%20ref%29))
  (if (Variables|Default|GetIsActive)
    (if (== OtherActor (Variables|Default|GetCharacter))
      (Utilities|FlowControl|DoOnce false :!label _label
        (:Completed
          (Physics|AddImpulse (Variables|Default|GetCollisionComponent) (* (Math|Vector|VectorUp) (Variables|Default|GetJumpStr)) "None" true)
          (Utilities|FlowControl|Delay 1.0)
          (CallFunction|ChaseCharacter)
          (goto _label Reset))))))

(event Custom|CustomEvent)

(event Custom|ChaseCharacter
  (AI|Navigation|SimpleMovetoLocation (AI|GetAIController self) (Transformation|GetActorLocation (Variables|Default|GetCharacter))))

(event EventBeginPlay
  (bind _returnvalue (Game|GetPlayerCharacter 0))
  (Utilities|IsValid _returnvalue
    (:Is%20Valid
      (Variables|Default|SetCharacter _returnvalue))))

(event Collision|EventActorBeginOverlap
  (params (OtherActor :type Actor%20Object%20Reference)))

(fn ConstructionScript
  (Components|Sphere|SetSphereRadius (Variables|Default|GetTrigger) (Variables|Default|GetIn%20Sphere%20Radius) true))