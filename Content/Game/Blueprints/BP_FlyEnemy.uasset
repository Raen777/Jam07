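; BP_FlyEnemy is an enemy that hops and chases the player character once it enters a configurable trigger sphere.
; Trigger overlap begin or end, gated by IsActive, starts a self-repeating loop: delay, upward impulse, then AI move to the player's location.
; A BP_Bullet hit clears IsActive, blocking new triggers, but the running loop never checks it.
; Leftover timer and teleport nodes are unconnected.
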(event OnComponentBeginOverlap(Trigger)
  (params (OverlappedComponent :type Primitive%20Component%20Object%20Reference) (OtherActor :type Actor%20Object%20Reference) (OtherComp :type Primitive%20Component%20Object%20Reference) (OtherBodyIndex :type Integer) (bFromSweep :type Boolean) (SweepResult :type Hit%20Result%20Structure%20%28by%20ref%29))
  (if (Variables|Default|GetIsActive)
    (if (== OtherActor (Variables|Default|GetCharacter))
      (Utilities|FlowControl|Delay 1.0)
      (Physics|AddImpulse (Variables|Default|GetCollisionComponent) (* (Math|Vector|VectorUp) (Variables|Default|GetJumpStr)) "None" true)
      (Utilities|FlowControl|Delay 0.4)
      (CallFunction|ChaseCharacter))))

(event OnComponentHit(MeshComponent)
  (params (HitComponent :type Primitive%20Component%20Object%20Reference) (OtherActor :type Actor%20Object%20Reference) (OtherComp :type Primitive%20Component%20Object%20Reference) (NormalImpulse :type Vector :default "0, 0, 0") (Hit :type Hit%20Result%20Structure%20%28by%20ref%29))
  (Utilities|Casting|CastToBP_Bullet OtherActor)
  (Variables|Default|SetIsActive false))

(event OnComponentEndOverlap(Trigger)
  (params (OverlappedComponent :type Primitive%20Component%20Object%20Reference) (OtherActor :type Actor%20Object%20Reference) (OtherComp :type Primitive%20Component%20Object%20Reference) (OtherBodyIndex :type Integer))
  (if (Variables|Default|GetIsActive)
    (if (== (stale OnComponentBeginOverlap(Trigger) OtherActor) (Variables|Default|GetCharacter))
      (Utilities|FlowControl|Delay 1.0)
      (Physics|AddImpulse (Variables|Default|GetCollisionComponent) (* (Math|Vector|VectorUp) (Variables|Default|GetJumpStr)) "None" true)
      (Utilities|FlowControl|Delay 0.4)
      (CallFunction|ChaseCharacter))))

(event Custom|CustomEvent)

(event Custom|ChaseCharacter
  (AI|Navigation|SimpleMovetoLocation (AI|GetAIController self) (Transformation|GetActorLocation (Variables|Default|GetCharacter)))
  (CallFunction|Repeat))

(event Custom|repeat
  (Utilities|FlowControl|Delay 1.0)
  (Physics|AddImpulse (Variables|Default|GetCollisionComponent) (* (Math|Vector|VectorUp) (Variables|Default|GetJumpStr)) "None" true)
  (Utilities|FlowControl|Delay 0.4)
  (CallFunction|ChaseCharacter))

(event EventBeginPlay
  (bind _returnvalue (Game|GetPlayerCharacter 0))
  (Utilities|IsValid _returnvalue
    (:Is%20Valid
      (Variables|Default|SetCharacter _returnvalue))))

(event Collision|EventActorBeginOverlap
  (params (OtherActor :type Actor%20Object%20Reference)))

(fn ConstructionScript
  (Components|Sphere|SetSphereRadius (Variables|Default|GetTrigger) (Variables|Default|GetIn%20Sphere%20Radius) true))