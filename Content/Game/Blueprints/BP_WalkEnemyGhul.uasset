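; BP_WalkEnemyGhul is a ghoul enemy that walks to noises and can be killed by bullets.
; PawnSensing noises make it run to the sound until it sees a pawn, which only sets a flag that blocks further noise responses.
; BP_Bullet hits subtract random HP, and mesh hits play an impact animation.
; At zero HP it plays a death animation once, unpossesses its AI controller and enables mesh physics.
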(event OnHearNoise(PawnSensing)
  (params (Instigator :type Pawn%20Object%20Reference) (Location :type Vector%20%28by%20ref%29 :default "0, 0, 0") (Volume :type Float%20%28single-precision%29))
  (if (not (Variables|Default|GetIsSeePlayer?))
    (AI|Navigation|SimpleMovetoLocation (Pawn|GetController) Location)
    (Components|Animation|PlayAnimation (Variables|Character|GetMesh) "/Game/Mobs/Mob_1_Demon/Anim/Demon_run_2_Anim.Demon_run_2_Anim" true)))

(event OnSeePawn(PawnSensing)
  (params (Pawn :type Pawn%20Object%20Reference))
  (Variables|Default|SetIsSeePlayer? true))

(event OnComponentHit(Mesh)
  (params (HitComponent :type Primitive%20Component%20Object%20Reference) (OtherActor :type Actor%20Object%20Reference) (OtherComp :type Primitive%20Component%20Object%20Reference) (NormalImpulse :type Vector :default "0, 0, 0") (Hit :type Hit%20Result%20Structure%20%28by%20ref%29))
  (Utilities|Casting|CastToBP_Bullet OtherActor)
  (Components|Animation|PlayAnimation (Variables|Character|GetMesh) "/Game/Mobs/Mob_1_Demon/Anim/Demon_impact_Anim.Demon_impact_Anim" false))

(event EventBeginPlay)

(event Collision|EventActorBeginOverlap
  (params (OtherActor :type Actor%20Object%20Reference)))

(event EventTick
  (params (DeltaSeconds :type Float%20%28single-precision%29)))

(event Collision|EventHit
  (params (MyComp :type Primitive%20Component%20Object%20Reference) (Other :type Actor%20Object%20Reference) (OtherComp :type Primitive%20Component%20Object%20Reference) (bSelfMoved :type Boolean) (HitLocation :type Vector :default "0, 0, 0") (HitNormal :type Vector :default "0, 0, 0") (NormalImpulse :type Vector :default "0, 0, 0") (Hit :type Hit%20Result%20Structure%20%28by%20ref%29))
  (bind _mesh (Variables|Character|GetMesh))
  (Utilities|Casting|CastToBP_Bullet Other)
  (bind _output_get (Variables|Default|SetHP (- (Variables|Default|GetHP) (Math|Random|RandomIntegerinRange 20 30))))
  (if (<= _output_get 0)
    (Utilities|FlowControl|DoOnce false
      (:Completed
        (Components|Animation|PlayAnimation _mesh "/Game/Mobs/Mob_1_Demon/Anim/Demon_Death_Anim.Demon_Death_Anim" false)
        (Pawn|UnPossess (AI|GetAIController self))
        (Utilities|FlowControl|Delay 0.0)
        (Physics|SetSimulatePhysics _mesh true)))))

(fn ConstructionScript
  (|CallParentFunction))